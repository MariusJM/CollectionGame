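; Game mode for a physics ball pickup game, handling levels, score, lives, timer, enemy spawning and end screens.
; Collectables add points and trigger growing pickup waves once all spawned are collected, until the win target slows time to zero.
; Rarity 8 pickups message all enemies through KillEnemyMessage, while enemy kills award points and respawn one after a delay.
; Deaths respawn and possess a new pawn until lives reach zero, showing game over.
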(event Custom|PickupsAndPointsCounter
  (params (Points :type Integer))
  ;[1 1 1] Game Loop
  ;;[1 1 1] Pickups and Points counter
  (Variables|Default|SetGamePoints (+ Points (Variables|Default|GetGamePoints)))
  (bind _result (Math|Integer|IncrementInt (Variables|Default|GetCollected))
    (:%20%20
      (Variables|Default|SetCollected _result))))

(event Custom|SpawnEnemy
  ;[1 1 1] SpawnEnemy
  (Game|SpawnActorfromClass "/Game/Blueprints/Enemies/BP_Enemy.BP_Enemy_C" (Math|Transform|MakeTransform "150.000000,150.000000,100.000000" "0, 0, 0" "1.000000,1.000000,1.000000") "AdjustIfPossibleButAlwaysSpawn" 0 0))

(event Custom|Add%20HUD
  ;[0.9922 0.9922 0.5569 0.8118] HUD Widget
  (bind _returnvalue (UserInterface|CreateWidget "/Game/UI/HUD/W_GameplayHUD.W_GameplayHUD_C"))
  (UserInterface|Viewport|AddtoViewport _returnvalue 0))

(event Custom|Start%20Timer
  ;[0.9922 0.9922 0.5569 0.8118] Timer
  (bind _newtrack_0 (Timeline|Timeline Play)
    (:Update
      (Variables|Default|SetTimer _newtrack_0))))

(event Custom|Stop%20Timer
  ;[0.9922 0.9922 0.5569 0.8118] Timer
  (bind _newtrack_0 (Timeline|Timeline Stop)
    (:Update
      (Variables|Default|SetTimer _newtrack_0))))

(event Custom|Next%20Level
  ;[1 1 1] Next Level / New pickups spawn
  (bind _output_get (Variables|Default|SetNextLevelPickupsToSpawn (+ (Variables|Default|GetNextLevelPickupsToSpawn) (Variables|Default|GetNextLevelPickupsIncrement))))
  (bind _returnvalue (Actor|GetActorOfClass "/Game/Blueprints/Pickup/BP_PickupSpawner.BP_PickupSpawner_C"))
  (Class|BPISpawnPickups|SpawnPickups(Message) _returnvalue _output_get)
  (Variables|Default|SetPickupsSpawnedAll (+ _output_get (Variables|Default|GetPickupsSpawnedAll)))
  (bind _result (Math|Integer|IncrementInt (Variables|Default|GetLevel))
    (:%20%20
      (Variables|Default|SetLevel _result))))

(event Custom|Win%20Screen
  (bind _returnvalue (Game|GetPlayerController 0))
  ;[1 1 1] Win Screen
  (CallFunction|StopTimer)
  (bind _returnvalue_2 (UserInterface|CreateWidget "/Game/UI/MainMenu/W_Win.W_Win_C"))
  (UserInterface|Viewport|AddtoViewport _returnvalue_2 0)
  (Variables|/Script/Engine.PlayerController|SetbShowMouseCursor _returnvalue true)
  (Input|SetInputModeUIOnly _returnvalue _returnvalue_2 "DoNotLock" false)
  (bind _newtrack_0 (Timeline|Timeline_0 PlayFromStart)
    (:Update
      (Utilities|Time|SetGlobalTimeDilation (Math|Float|Lerp 1.0 0.0 _newtrack_0)))))

(event Custom|EnemyVulnerable
  (params (RarityIndex :type Integer))
  ;[1 1 1] Game Loop
  (if (== RarityIndex 8)
    (bind _outactors (Actor|GetAllActorsOfClass "/Game/Blueprints/Enemies/BP_Enemy.BP_Enemy_C"))
    (Class|BPIKillEnemy|KillEnemy(Message) _outactors)))

(event Custom|RespawnEnemy
  ;[1 1 1] SpawnEnemy
  (Utilities|FlowControl|Delay 0.2)
  (Game|SpawnActorfromClass "/Game/Blueprints/Enemies/BP_Enemy.BP_Enemy_C" (Math|Transform|MakeTransform "150.000000,150.000000,100.000000" "0, 0, 0" "1.000000,1.000000,1.000000") "AdjustIfPossibleButAlwaysSpawn" 0 0))

(event EventBeginPlay
  ;[0.3545 1 0.3058] Initialization
  (CallFunction|AddHUD)
  (CallFunction|NextLevel)
  (CallFunction|StartTimer)
  (Input|SetInputModeGameOnly (Game|GetPlayerController 0) false)
  (CallFunction|SpawnEnemy))

(event EventCollectable
  (params (Points :type Integer) (RarityIndex :type Integer))
  ;[1 1 1] Game Loop
  (CallFunction|PickupsandPointsCounter Points)
  (CallFunction|EnemyVulnerable RarityIndex)
  (if (!= (Variables|Default|GetCollected) (Variables|Default|GetPickupsToWin))
    (if (not (!= (Variables|Default|GetPickupsSpawnedAll) (Variables|Default|GetCollected)))
      (CallFunction|NextLevel))
    (else
      (CallFunction|WinScreen))))

(event EventKillPlayer
  (bind _returnvalue (Game|GetPlayerController 0))
  ;[1 1 1] Kill Player Logic
  (bind _result (Math|Integer|DecrementInt (Variables|Default|GetLives))
    (:%20%20
      (bind _output_get (Variables|Default|SetLives _result))
      (if (== _output_get 0)
        (CallFunction|StopTimer)
        (bind _returnvalue_2 (UserInterface|CreateWidget "/Game/UI/MainMenu/W_GameOver.W_GameOver_C"))
        (UserInterface|Viewport|AddtoViewport _returnvalue_2 0)
        (Input|SetInputModeUIOnly _returnvalue _returnvalue_2 "DoNotLock" false)
        (Variables|/Script/Engine.PlayerController|SetbShowMouseCursor _returnvalue true)
        (else
          ;;[1 1 1] Respawn Pawn
          (bind _returnvalue_3 (Game|SpawnActorfromClass "/Game/Character/BP_MainPawn.BP_MainPawn_C" (Math|Transform|MakeTransform "0.000000,0.000000,100.000000" "0, 0, 0" "1.000000,1.000000,1.000000") "AdjustIfPossibleButAlwaysSpawn" 0 0))
          (Pawn|Possess (Game|GetPlayerController 0) _returnvalue_3))))))

(event EventKillEnemyPoints
  (params (Points :type Integer))
  ;[1 1 1] Game Loop
  ;;[1 1 1] Pickups and Points counter
  (Variables|Default|SetGamePoints (+ Points (Variables|Default|GetGamePoints)))
  (CallFunction|RespawnEnemy))

(fn ConstructionScript)