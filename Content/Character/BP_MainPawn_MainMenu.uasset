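; BP_MainPawn_MainMenu is the main menu version of the main pawn, animating its Sphere component with a continuous spin and hover.
; BeginPlay starts two timelines, each restarted by its own custom event when finished, forming endless loops.
; The Rotation timeline adds local yaw each update, while the second adds a small local Z offset interpolated from its Hover track.
; Both apply per-update deltas rather than absolute transforms.
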(event Custom|PlayRotationAnimation
  (bind _zrotation (Timeline|Rotation PlayFromStart)
    (:Update
      (Transformation|AddLocalRotation (Variables|Default|GetSphere) (Math|Rotator|MakeRotator 0.0 0.0 _zrotation) false false))
    (:Finished
      (CallFunction|PlayRotationAnimation))))

(event Custom|PlayHoveringAnimation
  (bind _hover (Timeline|Timeline PlayFromStart)
    (:Update
      (Class|SceneComponent|AddLocalTransform (Variables|Default|GetSphere) (Math|Transform|MakeTransform (Math|Vector|MakeVector 0.0 0.0 (Math|Float|Lerp -0.2 0.2 _hover)) "0, 0, 0" "1.000000,1.000000,1.000000") false false))
    (:Finished
      (CallFunction|PlayHoveringAnimation))))

(event EventBeginPlay
  (CallFunction|PlayRotationAnimation)
  (CallFunction|PlayHoveringAnimation))

(fn ConstructionScript)