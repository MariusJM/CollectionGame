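; Player pawn: a physics-driven ball that collects pickups for points, with HUD, stopwatch and pause menu.
; Enhanced Input adds camera-relative forces with clamped velocity, drives look and spring-arm zoom, and gates jumps through a DoOnce reset by a timeline.
; BeginPlay copies session stats from the game instance; overlaps notify BPI_Collectable actors and add score.
; Construction takes mesh and material from DT_Char_Dev, storing physics properties whose setters are unwired.
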(event OnComponentBeginOverlap(SM_Sphere)
  (params (OverlappedComponent :type Primitive%20Component%20Object%20Reference) (OtherActor :type Actor%20Object%20Reference) (OtherComp :type Primitive%20Component%20Object%20Reference) (OtherBodyIndex :type Integer) (bFromSweep :type Boolean) (SweepResult :type Hit%20Result%20Structure%20%28by%20ref%29))
  ;[1 1 1] Overlap with pickup
  ;;[1 1 1] Pickup destroy
  (if (Utilities|DoesObjectImplementInterface OtherActor "/Game/Blueprints/Pickup/BPI_Collectable.BPI_Collectable_C")
    (Class|BPICollectable|Collectable(Message) OtherActor)
    ;;[1 1 1] Collected pickup
    (bind _result (Math|Integer|IncrementInt (Variables|Default|GetCollected))
      (:%20%20
        (Variables|Default|SetCollected _result)
        (Variables|Default|SetGamePoints (+ (Variables|Default|GetGamePoints) 100))))))

(event Input|EnhancedActionEvents|EnhancedInputActionIA_Move
  (params (ActionValue :type Vector%202D%20Structure) (ElapsedSeconds :type Float%20%28double-precision%29) (TriggeredSeconds :type Float%20%28double-precision%29) (InputAction :type Input%20Action%20Object%20Reference :default "/Game/Game/Input/Actions/IA_Move.IA_Move"))
  (bind _camera (Variables|Default|GetCamera))
  (bind _returnvalue (Math|Vector|GetForwardVector _camera))
  (:Triggered
    (Physics|AddForce (Variables|Default|GetSM_Sphere) (* (Math|Vector|GetRightVector (Variables|Default|GetCamera)) (* (.x ActionValue) (Variables|Default|GetForce))) "None" true)
    (Physics|AddForce (Variables|Default|GetSM_Sphere) (* (Math|Vector|MakeVector (.x _returnvalue) (.y _returnvalue) 0.0) (* (.y ActionValue) (Variables|Default|GetForce))) "None" true)
    (bind _returnvalue_2 (Physics|GetPhysicsLinearVelocity (Variables|Default|GetSM_Sphere) "None"))
    (Physics|SetPhysicsLinearVelocity (Variables|Default|GetSM_Sphere) (Class|KismetMathLibrary|VectorClampSizeMax2D _returnvalue_2 1e+01) false "None")))

(event Input|EnhancedActionEvents|EnhancedInputActionIA_Look
  (params (ActionValue :type Vector%202D%20Structure) (ElapsedSeconds :type Float%20%28double-precision%29) (TriggeredSeconds :type Float%20%28double-precision%29) (InputAction :type Input%20Action%20Object%20Reference :default "/Game/Game/Input/Actions/IA_Look.IA_Look"))
  (:Triggered
    (Pawn|Input|AddControllerYawInput (.x ActionValue))
    (Pawn|Input|AddControllerPitchInput (* (.y ActionValue) -1.0))))

(event Input|EnhancedActionEvents|EnhancedInputActionIA_Jump
  (params (ActionValue :type Boolean) (ElapsedSeconds :type Float%20%28double-precision%29) (TriggeredSeconds :type Float%20%28double-precision%29) (InputAction :type Input%20Action%20Object%20Reference :default "/Game/Game/Input/Actions/IA_Jump.IA_Jump"))
  (:Triggered
    (Utilities|FlowControl|DoOnce false :!label _label
      (:Completed
        (Physics|AddForce (Variables|Default|GetSM_Sphere) (Math|Vector|MakeVector 0.0 0.0 5e+04) "None" true)
        (Timeline|Timeline PlayFromStart
          (:Finished
            (goto _label Reset)))))))

(event Input|EnhancedActionEvents|EnhancedInputActionIA_Zoom
  (params (ActionValue :type Float%20%28double-precision%29) (ElapsedSeconds :type Float%20%28double-precision%29) (TriggeredSeconds :type Float%20%28double-precision%29) (InputAction :type Input%20Action%20Object%20Reference :default "/Game/Game/Input/Actions/IA_Zoom.IA_Zoom"))
  (:Triggered
    (Variables|/Script/Engine.SpringArmComponent|SetTargetArmLength (Variables|Default|GetSpringArm) (Math|Float|Clamp(Float) (+ (Variables|/Script/Engine.SpringArmComponent|GetTargetArmLength (Variables|Default|GetSpringArm)) (* (Math|Float|Clamp(Float) (* ActionValue -1.0) -1.0) 5e+01)) 3e+02 1e+03))))

(event Input|EnhancedActionEvents|EnhancedInputActionIA_Escape
  (params (ActionValue :type Boolean) (ElapsedSeconds :type Float%20%28double-precision%29) (TriggeredSeconds :type Float%20%28double-precision%29) (InputAction :type Input%20Action%20Object%20Reference :default "/Game/Game/Input/Actions/IA_Escape.IA_Escape"))
  (:Triggered
    (Game|SetGamePaused true)
    (bind _returnvalue (UserInterface|CreateWidget "/Game/UI/MainMenu/W_MM_Pause.W_MM_Pause_C"))
    (UserInterface|Viewport|AddtoViewport _returnvalue 0)
    (Input|SetInputModeGameandUI (Game|GetPlayerController 0) _returnvalue "DoNotLock" true false)))

(event EventBeginPlay
  (CallFunction|InputsBinds)
  (CallFunction|GetDatafromGameInstance)
  ;[1 1 1] HUD and timer
  (bind _returnvalue (UserInterface|CreateWidget "/Game/UI/HUD/W_GameplayHUD.W_GameplayHUD_C"))
  (UserInterface|Viewport|AddtoViewport _returnvalue 0)
  (bind _newtrack_0 (Timeline|Stopwatch Play)
    (:Update
      (Variables|Default|SetTimer _newtrack_0)
      (Variables|Default|SetGlobalTime _newtrack_0))))

(event EventTick
  (params (DeltaSeconds :type Float%20%28single-precision%29)))

(fn ConstructionScript
  (bind _sm_sphere (Variables|Default|GetSM_Sphere))
  ;[1 1 1] Ged Data
  (bind _returnvalue (Utilities|GetDataTableRow "/Game/Data/Character/DT_Char_Dev.DT_Char_Dev" "DevCharacter")
    (:then
      (Components|StaticMesh|SetStaticMesh _sm_sphere (.StaticMesh (Utilities|Struct|BreakStr_Char_Dev _returnvalue)))
      (Rendering|Material|SetMaterial _sm_sphere 0 (.Material (Utilities|Struct|BreakStr_Char_Dev _returnvalue)))
      (Variables|Default|SetCharPhysicsProperties (.PhysicsProperties (Utilities|Struct|BreakStr_Char_Dev _returnvalue))))))

(fn GetDatafromGameInstance
  (bind _asgi_boiafgameinstance (Utilities|Casting|CastToGI_BOIAFGameinstance (Game|GetGameInstance)))
  (Variables|Default|SetGlobalTime (Variables|/Game/Game/GI_BOIAFGameinstance.GI_BOIAFGameinstance_C|GetGIv_GlobalTime _asgi_boiafgameinstance))
  (Variables|Default|SetPickups (Variables|/Game/Game/GI_BOIAFGameinstance.GI_BOIAFGameinstance_C|GetGIv_PickupsSpawn _asgi_boiafgameinstance))
  (Variables|Default|SetLives (Variables|/Game/Game/GI_BOIAFGameinstance.GI_BOIAFGameinstance_C|GetGIv_Lives _asgi_boiafgameinstance))
  (Variables|Default|SetGamePoints (Variables|/Game/Game/GI_BOIAFGameinstance.GI_BOIAFGameinstance_C|GetGIv_GamePoints _asgi_boiafgameinstance))
  (Variables|Default|SetLevel (Variables|/Game/Game/GI_BOIAFGameinstance.GI_BOIAFGameinstance_C|GetGIv_Level _asgi_boiafgameinstance)))

(fn InputsBinds
  (bind _asplayer_controller (Utilities|Casting|CastToPlayerController (Pawn|GetController)))
  (Input|AddMappingContext (PlayerController|LocalPlayerSubsystems|GetEnhancedInputLocalPlayerSubsystem _asplayer_controller) "/Game/Game/Input/IMC_Default.IMC_Default" 0 "(bIgnoreAllPressedKeysUntilRelease=True,bForceImmediately=False)"))