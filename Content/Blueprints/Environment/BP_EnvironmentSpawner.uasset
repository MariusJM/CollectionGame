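; Procedurally builds a walled arena level at BeginPlay, sized from the Level_001_Map row of DT_Levels read in the construction script.
; BP_EnvironmentAsset actors form the scaled ground, four corner pillars and connecting walls, which reuse the pillar mesh and material.
; A 2D grid macro places platforms with random mesh and height in cells that pass a 25% roll.
; A pickup spawner above the arena and an oversized kill box below complete it.
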(event Custom|Spawn%20Ground
  (bind _ground (Variables|Default|GetGround))
  (bind _returnvalue (Game|SpawnActorfromClass "/Game/Blueprints/Environment/BP_EnvironmentAsset.BP_EnvironmentAsset_C" (Variables|Default|GetSpawn%20Transform) "Undefined" 0 0))
  (bind _output_get (Variables|Default|SetSpawn%20Transform (Math|Transform|MakeTransform "0, 0, 0" "0, 0, 0" (Math|Vector|MakeVector (.groundsizex _ground) (.groundsizey _ground) 1.0))))
  (Default|ConstructGround _returnvalue (.groundmesh _ground) (.groundmaterial _ground) _output_get))

(event Custom|Spawn%20Pillars
  (bind _pillar (Variables|Default|GetPillar))
  (bind _pillar_2 (Variables|Default|GetPillar))
  (bind _pillar_3 (Variables|Default|GetPillar))
  (bind _ground (Variables|Default|GetGround))
  (bind _pillar_4 (Variables|Default|GetPillar))
  (Utilities|FlowControl|Sequence
    (:then_0
      (bind _returnvalue (Game|SpawnActorfromClass "/Game/Blueprints/Environment/BP_EnvironmentAsset.BP_EnvironmentAsset_C" (Math|Transform|MakeTransform "0, 0, 0" "0, 0, 0" "1.000000,1.000000,1.000000") "Undefined" 0 0))
      (bind _output_get (Variables|Default|SetSpawn%20Transform (Math|Transform|MakeTransform "0, 0, 0" "0, 0, 0" (Math|Vector|MakeVector (.pillarsizex _pillar) (.pillarsizey _pillar) (.pillarsizez _pillar)))))
      (Default|ConstructPillar _returnvalue (.pillarmesh _pillar) (.pillarmaterial _pillar) _output_get))
    (:then_1
      (bind _returnvalue_2 (Game|SpawnActorfromClass "/Game/Blueprints/Environment/BP_EnvironmentAsset.BP_EnvironmentAsset_C" (Math|Transform|MakeTransform "0, 0, 0" "0, 0, 0" "1.000000,1.000000,1.000000") "Undefined" 0 0))
      (bind _output_get_2 (Variables|Default|SetSpawn%20Transform (Math|Transform|MakeTransform (Math|Vector|MakeVector (* (.groundsizex (Variables|Default|GetGround)) 1e+02) 0.0 0.0) "0.000000,-90.000000,0.000000" (Math|Vector|MakeVector (.pillarsizex _pillar_2) (.pillarsizey _pillar_2) (.pillarsizez _pillar_2)))))
      (Default|ConstructPillar _returnvalue_2 (.pillarmesh _pillar_2) (.pillarmaterial _pillar_2) _output_get_2))
    (:then_2
      (bind _returnvalue_3 (Game|SpawnActorfromClass "/Game/Blueprints/Environment/BP_EnvironmentAsset.BP_EnvironmentAsset_C" (Math|Transform|MakeTransform "0, 0, 0" "0, 0, 0" "1.000000,1.000000,1.000000") "Undefined" 0 0))
      (bind _output_get_3 (Variables|Default|SetSpawn%20Transform (Math|Transform|MakeTransform (Math|Vector|MakeVector (* (.groundsizex _ground) 1e+02) (* (.groundsizey _ground) -1e+02) 0.0) "0.000000,180.000000,0.000000" (Math|Vector|MakeVector (.pillarsizex _pillar_3) (.pillarsizey _pillar_3) (.pillarsizez _pillar_3)))))
      (Default|ConstructPillar _returnvalue_3 (.pillarmesh _pillar_3) (.pillarmaterial _pillar_3) _output_get_3))
    (:then_3
      (bind _returnvalue_4 (Game|SpawnActorfromClass "/Game/Blueprints/Environment/BP_EnvironmentAsset.BP_EnvironmentAsset_C" (Math|Transform|MakeTransform "0, 0, 0" "0, 0, 0" "1.000000,1.000000,1.000000") "Undefined" 0 0))
      (bind _output_get_4 (Variables|Default|SetSpawn%20Transform (Math|Transform|MakeTransform (Math|Vector|MakeVector 0.0 (* (.groundsizey (Variables|Default|GetGround)) -1e+02) 0.0) "0.000000,90.000000,0.000000" (Math|Vector|MakeVector (.pillarsizex _pillar_4) (.pillarsizey _pillar_4) (.pillarsizez _pillar_4)))))
      (Default|ConstructPillar _returnvalue_4 (.pillarmesh _pillar_4) (.pillarmaterial _pillar_4) _output_get_4))))

(event Custom|Spawn%20Walls
  (bind _pillar (Variables|Default|GetPillar))
  (bind _ground (Variables|Default|GetGround))
  (bind _wall (Variables|Default|GetWall))
  (bind _pillar_2 (Variables|Default|GetPillar))
  (bind _wall_2 (Variables|Default|GetWall))
  (bind _pillar_3 (Variables|Default|GetPillar))
  (bind _pillar_4 (Variables|Default|GetPillar))
  (bind _ground_2 (Variables|Default|GetGround))
  (bind _wall_3 (Variables|Default|GetWall))
  (bind _pillar_5 (Variables|Default|GetPillar))
  (bind _pillar_6 (Variables|Default|GetPillar))
  (bind _ground_3 (Variables|Default|GetGround))
  (bind _wall_4 (Variables|Default|GetWall))
  (bind _pillar_7 (Variables|Default|GetPillar))
  (Utilities|FlowControl|Sequence
    (:then_0
      (bind _returnvalue (Game|SpawnActorfromClass "/Game/Blueprints/Environment/BP_EnvironmentAsset.BP_EnvironmentAsset_C" (Math|Transform|MakeTransform "0, 0, 0" "0, 0, 0" "1.000000,1.000000,1.000000") "Undefined" 0 0))
      (bind _output_get (Variables|Default|SetSpawn%20Transform (Math|Transform|MakeTransform (Math|Vector|MakeVector (* (.pillarsizex _pillar_2) 1e+02) 0.0 0.0) "0, 0, 0" (Math|Vector|MakeVector (- (.groundsizex (Variables|Default|GetGround)) (+ (.pillarsizex _pillar_2) (.pillarsizey _pillar_2))) (.wallthickness _wall_2) (.wallheight _wall_2)))))
      (Default|ConstructWall _returnvalue (.pillarmesh _pillar_2) (.pillarmaterial _pillar_2) _output_get))
    (:then_1
      (bind _returnvalue_2 (Game|SpawnActorfromClass "/Game/Blueprints/Environment/BP_EnvironmentAsset.BP_EnvironmentAsset_C" (Math|Transform|MakeTransform "0, 0, 0" "0, 0, 0" "1.000000,1.000000,1.000000") "Undefined" 0 0))
      (bind _output_get_2 (Variables|Default|SetSpawn%20Transform (Math|Transform|MakeTransform (Math|Vector|MakeVector (* (.groundsizex _ground_2) 1e+02) (* (.pillarsizey _pillar_4) -1e+02) 0.0) "0.000000,-90.000000,0.000000" (Math|Vector|MakeVector (- (.groundsizey _ground_2) (+ (.pillarsizex _pillar_4) (.pillarsizey _pillar_4))) (.wallthickness _wall_3) (.wallheight _wall_3)))))
      (Default|ConstructWall _returnvalue_2 (.pillarmesh _pillar_5) (.pillarmaterial _pillar_5) _output_get_2))
    (:then_2
      (bind _returnvalue_3 (Game|SpawnActorfromClass "/Game/Blueprints/Environment/BP_EnvironmentAsset.BP_EnvironmentAsset_C" (Math|Transform|MakeTransform "0, 0, 0" "0, 0, 0" "1.000000,1.000000,1.000000") "Undefined" 0 0))
      (bind _output_get_3 (Variables|Default|SetSpawn%20Transform (Math|Transform|MakeTransform (Math|Vector|MakeVector (- (* (.groundsizex _ground_3) 1e+02) (* (.pillarsizex _pillar_6) 1e+02)) (* (.groundsizey _ground_3) -1e+02) 0.0) "0.000000,180.000000,0.000000" (Math|Vector|MakeVector (- (.groundsizex _ground_3) (+ (.pillarsizex _pillar_6) (.pillarsizey _pillar_6))) (.wallthickness _wall_4) (.wallheight _wall_4)))))
      (Default|ConstructWall _returnvalue_3 (.pillarmesh _pillar_7) (.pillarmaterial _pillar_7) _output_get_3))
    (:then_3
      (bind _returnvalue_4 (Game|SpawnActorfromClass "/Game/Blueprints/Environment/BP_EnvironmentAsset.BP_EnvironmentAsset_C" (Math|Transform|MakeTransform "0, 0, 0" "0, 0, 0" "1.000000,1.000000,1.000000") "Undefined" 0 0))
      (bind _output_get_4 (Variables|Default|SetSpawn%20Transform (Math|Transform|MakeTransform (Math|Vector|MakeVector 0.0 (+ (* (.groundsizey _ground) -1e+02) (* (.pillarsizex _pillar_3) 1e+02)) 0.0) "0.000000,90.000000,0.000000" (Math|Vector|MakeVector (- (.groundsizey _ground) (+ (.pillarsizex _pillar_3) (.pillarsizey _pillar_3))) (.wallthickness _wall) (.wallheight _wall)))))
      (Default|ConstructWall _returnvalue_4 (.pillarmesh _pillar) (.pillarmaterial _pillar) _output_get_4))))

(event Custom|Spawn%20Spawner
  (bind _ground (Variables|Default|GetGround))
  (bind _ground_2 (Variables|Default|GetGround))
  (bind _pillar (Variables|Default|GetPillar))
  (bind _returnvalue (Game|SpawnActorfromClass "/Game/Blueprints/Pickup/BP_PickupSpawner.BP_PickupSpawner_C" (Math|Transform|MakeTransform (Math|Vector|MakeVector (* (.groundsizex _ground_2) 5e+01) (* (.groundsizey _ground_2) -5e+01) (* (* (.wallheight (Variables|Default|GetWall)) 1e+02) 2.0)) "0, 0, 0" "1.000000,1.000000,1.000000") "Undefined" 0 0))
  (Components|Box|SetBoxExtent (Variables|/Game/Blueprints/Pickup/BP_PickupSpawner.BP_PickupSpawner_C|GetBox _returnvalue) (Math|Vector|MakeVector (* (- (.groundsizex _ground) (* (.pillarsizex _pillar) 2.0)) 5e+01) (* (- (.groundsizey _ground) (* (.pillarsizey _pillar) 2.0)) 5e+01) 2e+02) true))

(event Custom|Spawn%20Platforms
  (bind _platform (Variables|Default|GetPlatform))
  (bind _platform_2 (Variables|Default|GetPlatform))
  (bind _platform_3 (Variables|Default|GetPlatform))
  (bind _ground (Variables|Default|GetGround))
  (bind _pillar (Variables|Default|GetPillar))
  (bind _returnvalue (* (.platformsizex _platform_3) 1e+02))
  (bind _poly_center (Utilities|2DGridExecutionMacro _returnvalue (Math|Vector|MakeVector (+ (/ _returnvalue 2.0) (/ (.groundsizex _ground) 0.02)) (+ (/ (.groundsizey _ground) -0.02) (/ (* (.platformsizey _platform_3) 1e+02) -2.0)) 0.0) (Math|Float|Truncate (/ (- (.groundsizex _ground) (* (.pillarsizex _pillar) 2.0)) (.platformsizex _platform_3))) (Math|Float|Truncate (/ (- (.groundsizey _ground) (* (.pillarsizey _pillar) 2.0)) (.platformsizey _platform_3))))
    (:Per%20Poly%20Execution
      (if (Math|Random|RandomBoolwithWeight 0.25)
        (bind _returnvalue_2 (Game|SpawnActorfromClass "/Game/Blueprints/Environment/BP_EnvironmentAsset.BP_EnvironmentAsset_C" (Math|Transform|MakeTransform _poly_center "0.000000,180.000000,0.000000" (Math|Vector|MakeVector (.platformsizex _platform_2) (.platformsizey _platform_2) (* (.OutItem (Utilities|Array|Random (.platformsizezarray _platform_2))) 2.0))) "Undefined" 0 0))
        (Default|ConstructPlatform _returnvalue_2 (.OutItem (Utilities|Array|Random (.platformmesh _platform))) (.platformmaterial _platform))))))

(event Custom|SpawnKillBox
  (bind _ground (Variables|Default|GetGround))
  (Game|SpawnActorfromClass "/Game/Blueprints/KillPlayer/BP_KillBox.BP_KillBox_C" (Math|Transform|MakeTransform (Math|Vector|MakeVector (* (.groundsizex _ground) 5e+01) (* (.groundsizey _ground) -5e+01) -1e+02) "0, 0, 0" (Math|Vector|MakeVector (* (.groundsizex _ground) 3.0) (* (.groundsizey _ground) 3.0) 1.0)) "Undefined" 0 0))

(event EventBeginPlay
  (Utilities|FlowControl|Sequence
    (:then_0
      (CallFunction|SpawnGround))
    (:then_1
      (CallFunction|SpawnPillars))
    (:then_2
      (CallFunction|SpawnWalls))
    (:then_3
      (CallFunction|SpawnPlatforms))
    (:then_4
      (CallFunction|SpawnSpawner))
    (:then_5
      (CallFunction|SpawnKillBox))))

(fn ConstructionScript
  (bind _returnvalue (Utilities|GetDataTableRow "/Game/Data/Levels/DT_Levels.DT_Levels" "Level_001_Map")
    (:then
      (Variables|Default|SetGround (.Ground (Utilities|Struct|BreakStr_Levels _returnvalue)))
      (Variables|Default|SetPillar (.Pillar (Utilities|Struct|BreakStr_Levels _returnvalue)))
      (Variables|Default|SetWall (.Wall (Utilities|Struct|BreakStr_Levels _returnvalue)))
      (Variables|Default|SetPlatform (.Platform (Utilities|Struct|BreakStr_Levels _returnvalue))))))