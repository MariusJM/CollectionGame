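; BP_EnvironmentAsset is a generic environment piece that takes on the role of ground, pillar, wall or platform through its single StaticMesh component.
; Ground, pillar and wall events pass a mesh, material and transform to a shared SetParameters function, which applies them, placing the component in world space.
; The platform event sets only mesh and first-slot material, leaving the transform untouched.
; The construction script is empty, so setup relies on these events being called.
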(event Custom|Construct%20Ground
  (params (Ground%20Mesh :type Static%20Mesh%20Object%20Reference) (Ground%20Material :type Material%20Instance%20Object%20Reference) (SpawnTransform :type Transform))
  (CallFunction|SetParameters Ground%20Mesh Ground%20Material SpawnTransform))

(event Custom|Construct%20Pillar
  (params (Mesh :type Static%20Mesh%20Object%20Reference) (Material :type Material%20Instance%20Object%20Reference) (Transform :type Transform))
  (CallFunction|SetParameters Mesh Material Transform))

(event Custom|Construct%20Wall
  (params (Mesh :type Static%20Mesh%20Object%20Reference) (Material :type Material%20Instance%20Object%20Reference) (Transform :type Transform))
  (CallFunction|SetParameters Mesh Material Transform))

(event Custom|Construct%20Platform
  (params (Mesh :type Static%20Mesh%20Object%20Reference) (Material :type Material%20Instance%20Object%20Reference))
  (bind _staticmesh (Variables|Default|GetStaticMesh))
  (Components|StaticMesh|SetStaticMesh _staticmesh Mesh)
  (Rendering|Material|SetMaterial _staticmesh 0 Material))

(fn ConstructionScript)

(fn SetParameters
  (params (Mesh :type Static%20Mesh%20Object%20Reference) (Material :type Material%20Instance%20Object%20Reference) (Transform :type Transform))
  (bind _staticmesh (Variables|Default|GetStaticMesh))
  (Components|StaticMesh|SetStaticMesh _staticmesh Mesh)
  (Rendering|Material|SetMaterial _staticmesh 0 Material)
  (Transformation|SetWorldTransform _staticmesh Transform false false))