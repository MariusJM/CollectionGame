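; BP_Respawn is a box trigger volume that sends a death message to respawnable actors entering it.
; On overlap, it checks whether the other actor implements BPI_Respawner and calls DeathMessage through that interface, leaving the response to that actor.
; The construction script scales the box from its size variables and shifts it upward in proportion to its height.
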(event OnComponentBeginOverlap(Box)
  (params (OverlappedComponent :type Primitive%20Component%20Object%20Reference) (OtherActor :type Actor%20Object%20Reference) (OtherComp :type Primitive%20Component%20Object%20Reference) (OtherBodyIndex :type Integer) (bFromSweep :type Boolean) (SweepResult :type Hit%20Result%20Structure%20%28by%20ref%29))
  (if (Utilities|DoesObjectImplementInterface OtherActor "/Game/Blueprints/BPI_Respawner.BPI_Respawner_C")
    (Class|BPIRespawner|Death(Message) OtherActor)))

(fn ConstructionScript
  (bind _box (Variables|Default|GetBox))
  (bind _returnvalue (Transformation|GetWorldLocation _box))
  (Transformation|SetRelativeScale3D _box (Math|Vector|MakeVector (Variables|Default|GetSize%20X) (Variables|Default|GetSize%20Y) (Variables|Default|GetSize%20Z)))
  (Transformation|SetWorldLocation _box (Math|Vector|MakeVector (.x _returnvalue) (.y _returnvalue) (+ (.z _returnvalue) (* (/ (Variables|Default|GetSize%20Z) 2.0) 5e+01))) false false))