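; BP_Platform is a resizable platform actor built from a central mesh and two side strip meshes.
; Its construction script scales the platform by ScaleX, ScaleY and ScaleZ, keeps both strips at a fixed thin width, and offsets the right strip to follow ScaleX.
; Dynamic material nodes for platform color, surface properties and strip emissive color exist but are disconnected, so they never run.
; The event graph holds no active logic.
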(event EventBeginPlay)

(event Collision|EventActorBeginOverlap
  (params (OtherActor :type Actor%20Object%20Reference)))

(event EventTick
  (params (DeltaSeconds :type Float%20%28single-precision%29)))

(fn ConstructionScript
  (bind _sm_sidestrip_r (Variables|Default|GetSM_SideStrip_R))
  (Transformation|SetRelativeScale3D (Variables|Default|GetSM_Platform) (Math|Vector|MakeVector (Variables|Default|GetScale_X) (Variables|Default|GetScale_Y) (Variables|Default|GetScale_Z)))
  (Transformation|SetRelativeScale3D (Variables|Default|GetSM_SideStrip_L) (Math|Vector|MakeVector 0.1 (Variables|Default|GetScale_Y) (Variables|Default|GetScale_Z)))
  (Transformation|SetRelativeScale3D _sm_sidestrip_r (Math|Vector|MakeVector 0.1 (Variables|Default|GetScale_Y) (Variables|Default|GetScale_Z)))
  (Transformation|SetRelativeLocation _sm_sidestrip_r (Math|Vector|MakeVector (+ (* (Variables|Default|GetScale_X) 1e+02) 1e+01) 0.0 0.0) false false))