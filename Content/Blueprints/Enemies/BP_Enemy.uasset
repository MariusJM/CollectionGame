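; Enemy pawn that kills the player on sphere overlap, or is destroyed for 500 points while vulnerable.
; KillEnemy starts the vulnerable state, with a timeline fading the dynamic material's emissive colour from inverted back to PrimaryColor.
; Pawn sensing and vulnerability write AI blackboard keys.
; The timeline's end clears IsVulnerable but sets the misspelled "IsVulnerabele" key to true again, so this Blueprint never resets that key.
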(event OnSeePawn(PawnSensing)
  (params (Pawn :type Pawn%20Object%20Reference))
  ;[1 1 1] AI Behavior
  (AI|Components|Blackboard|SetValueasBool (AI|GetBlackboard (AI|GetAIController self)) (Utilities|Name|MakeLiteralName "IsSeeingPlayer") true))

(event OnComponentBeginOverlap(SphereCollision)
  (params (OverlappedComponent :type Primitive%20Component%20Object%20Reference) (OtherActor :type Actor%20Object%20Reference) (OtherComp :type Primitive%20Component%20Object%20Reference) (OtherBodyIndex :type Integer) (bFromSweep :type Boolean) (SweepResult :type Hit%20Result%20Structure%20%28by%20ref%29))
  (bind _returnvalue (Game|GetGameMode))
  ;[1 1 1] Kill Player
  (if (Utilities|DoesObjectImplementInterface OtherActor "/Game/Blueprints/KillPlayer/BPI_KillPlayer.BPI_KillPlayer_C")
    (if (Variables|Default|GetIsVulnerable)
      (Actor|DestroyActor)
      (Class|BPIKillEnemy|KillEnemyPoints(Message) _returnvalue 500)
      (else
        (Class|BPIKillPlayer|KillPlayer(Message) OtherActor)
        (Class|BPIKillPlayer|KillPlayer(Message) _returnvalue)))))

(event EventKillEnemy
  (bind _self self)
  (bind _primarycolor (Variables|Default|GetPrimaryColor))
  (bind _returnvalue (AI|GetAIController _self))
  (bind _returnvalue_2 (- "(R=1.000000,G=1.000000,B=1.000000,A=1.000000)" _primarycolor))
  (bind _returnvalue_3 (AI|GetBlackboard _returnvalue))
  ;[1 1 1] Vulnerability
  (Rendering|Material|SetVectorParameterValue (Variables|Default|GetMIValue) "EmissiveColor" _returnvalue_2 :!class /Script/Engine.MaterialInstanceDynamic)
  (Variables|Default|SetIsVulnerable true)
  (AI|Components|Blackboard|SetValueasBool _returnvalue_3 (Utilities|Name|MakeLiteralName "IsVulnerabele") true)
  (bind _newtrack_0 (Timeline|VulnerableTimer PlayFromStart)
    (:Update
      (Rendering|Material|SetVectorParameterValue (Variables|Default|GetMIValue) "EmissiveColor" (Math|Color|Lerp(LinearColor) _returnvalue_2 (Variables|Default|GetPrimaryColor) _newtrack_0) :!class /Script/Engine.MaterialInstanceDynamic))
    (:Finished
      (Variables|Default|SetIsVulnerable false)
      (AI|Components|Blackboard|SetValueasBool _returnvalue_3 (Utilities|Name|MakeLiteralName "IsVulnerabele") true))))

(event EventBeginPlay
  ;[1 1 1] Initialization
  (bind _returnvalue (Rendering|Material|CreateDynamicMaterialInstance (Variables|Default|GetSphere) 0 0 "None" :!class /Script/Engine.PrimitiveComponent))
  (bind _output_get (Variables|Default|SetMIValue _returnvalue))
  (Rendering|Material|SetVectorParameterValue _output_get "EmissiveColor" (Variables|Default|GetPrimaryColor) :!class /Script/Engine.MaterialInstanceDynamic))

(fn ConstructionScript)